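; Creature Blueprint that builds a procedural skeletal body and lets the player extend it at runtime.
; On BeginPlay it enables input, has CreatureBodyMaker generate a mesh from Materials, assigns it to the PoseableMesh and sets a world-space rotation on bone s0in.
; Keys 0 and 1 add a bone to the body's end or front, then rerun that generation step to rebuild the mesh.
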(event EventBeginPlay
  (Input|EnableInput (Game|GetPlayerController 0))
  (bind _returnvalue (Class|CreatureBodyMaker|Generate (Variables|Default|GetCreatureBodyMaker) (Variables|Default|GetMaterials)))
  (Utilities|IsValid _returnvalue
    (:Is%20Valid
      (Class|SkinnedMeshComponent|SetSkeletalMesh (Variables|Default|GetPoseableMesh) _returnvalue true)
      (Components|PoseableMesh|SetBoneRotationbyName (Variables|Default|GetPoseableMesh) "s0in" "90.000000,0.300000,90.000000" "WorldSpace"))))

(event Collision|EventActorBeginOverlap
  (params (OtherActor :type Actor%20Object%20Reference)))

(event EventTick
  (params (DeltaSeconds :type Float%20%28single-precision%29)))

(event Input|KeyboardEvents|0
  (params (Key :type Key%20Structure :default "None"))
  (bind _creaturebodymaker (Variables|Default|GetCreatureBodyMaker))
  (:Pressed
    (Class|CreatureBodyMaker|AddBonetoBodyEnd _creaturebodymaker)
    (bind _returnvalue (Class|CreatureBodyMaker|Generate _creaturebodymaker (Variables|Default|GetMaterials)))
    (Utilities|IsValid _returnvalue
      (:Is%20Valid
        (Class|SkinnedMeshComponent|SetSkeletalMesh (Variables|Default|GetPoseableMesh) _returnvalue true)
        (Components|PoseableMesh|SetBoneRotationbyName (Variables|Default|GetPoseableMesh) "s0in" "90.000000,0.300000,90.000000" "WorldSpace")))))

(event Input|KeyboardEvents|1
  (params (Key :type Key%20Structure :default "None"))
  (bind _creaturebodymaker (Variables|Default|GetCreatureBodyMaker))
  (:Pressed
    (Class|CreatureBodyMaker|AddBonetoBodyFront _creaturebodymaker)
    (bind _returnvalue (Class|CreatureBodyMaker|Generate _creaturebodymaker (Variables|Default|GetMaterials)))
    (Utilities|IsValid _returnvalue
      (:Is%20Valid
        (Class|SkinnedMeshComponent|SetSkeletalMesh (Variables|Default|GetPoseableMesh) _returnvalue true)
        (Components|PoseableMesh|SetBoneRotationbyName (Variables|Default|GetPoseableMesh) "s0in" "90.000000,0.300000,90.000000" "WorldSpace")))))

(fn ConstructionScript)